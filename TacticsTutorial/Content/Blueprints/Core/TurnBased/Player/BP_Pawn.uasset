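; BP_Pawn is a camera pawn for the turn-based game, with zoom, movement and stepped rotation.
; Input events only update desired location, rotation and clamped spring-arm length, seeded from the starting state on BeginPlay.
; Tick eases the actor and spring arm toward those targets with interpolation for smooth motion.
; Both the Forward and Left axes move along the forward vector, with Left negated, so neither strafes sideways.
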(event EventTick
  (params (DeltaSeconds :type Float%20%28single-precision%29))
  (bind _springarm (Variables|Default|GetSpringArm))
  (Variables|/Script/Engine.SpringArmComponent|SetTargetArmLength _springarm (Math|Interpolation|FInterpTo (Variables|/Script/Engine.SpringArmComponent|GetTargetArmLength _springarm) (Variables|Default|GetDesiredZoom) DeltaSeconds 1.5))
  (Transformation|SetActorLocation (Math|Interpolation|VInterpTo (Transformation|GetActorLocation) (Variables|Default|GetLocation_desired) DeltaSeconds 1.5) false false)
  (Transformation|SetActorRotation (Math|Interpolation|RInterpTo (Transformation|GetActorRotation) (Variables|Default|GetRotation_desired) DeltaSeconds 2.0)))

(event EventBeginPlay
  (Variables|Default|SetLocation_desired (Transformation|GetActorLocation))
  (Variables|Default|SetDesiredZoom (Variables|/Script/Engine.SpringArmComponent|GetTargetArmLength (Variables|Default|GetSpringArm)))
  (Variables|Default|SetRotation_desired (Transformation|GetActorRotation)))

(event Input|ActionEvents|InputActioninputAction_RotateLeft
  (params (Key :type Key%20Structure :default "None"))
  (:Pressed
    (Variables|Default|SetRotation_desired (Math|Rotator|CombineRotators (Variables|Default|GetRotation_desired) "0.000000,-15.000000,0.000000"))))

(event Input|ActionEvents|InputActioninputAction_RotateRight
  (params (Key :type Key%20Structure :default "None"))
  (:Pressed
    (Variables|Default|SetRotation_desired (Math|Rotator|CombineRotators (Variables|Default|GetRotation_desired) "0.000000,15.000000,0.000000"))))

(event Input|AxisEvents|InputAxisinputAxis_Zoom
  (params (AxisValue :type Float%20%28single-precision%29))
  (Variables|Default|SetDesiredZoom (Math|Float|Clamp(Float) (+ AxisValue (Variables|Default|GetDesiredZoom)) 1e+02 5e+03)))

(event Input|AxisEvents|InputAxisinputAxis_Forward
  (params (AxisValue :type Float%20%28single-precision%29))
  (Variables|Default|SetLocation_desired (+ (Variables|Default|GetLocation_desired) (* (Transformation|GetActorForwardVector) (* AxisValue 25.0)))))

(event Input|AxisEvents|InputAxisinputAxis_Left
  (params (AxisValue :type Float%20%28single-precision%29))
  (Variables|Default|SetLocation_desired (+ (Variables|Default|GetLocation_desired) (* (Transformation|GetActorForwardVector) (* AxisValue -25.0)))))

(fn ConstructionScript)